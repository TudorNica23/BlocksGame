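; BP_Block is a block actor that can be gradually destroyed, with destruction shown through its material.
; On BeginPlay it creates a dynamic material instance from the block mesh and sets the timeline speed from DestroyRate.
; StartDestroy plays a timeline that drives the DestroyAmount scalar parameter and destroys the actor when it finishes.
; StopDestroy resets that parameter to zero and halts the timeline.
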(event Custom|Start%20Destroy
  (bind _destroyamount (Timeline|DestroyTimeline Play)
    (:Update
      (Rendering|Material|SetScalarParameterValue (Variables|Default|GetBlocMat) "DestroyAmount" _destroyamount :!class /Script/Engine.MaterialInstanceDynamic))
    (:Finished
      (Actor|DestroyActor))))

(event Custom|Stop%20Destroy
  (Rendering|Material|SetScalarParameterValue (Variables|Default|GetBlocMat) "DestroyAmount" 0.0 :!class /Script/Engine.MaterialInstanceDynamic)
  (bind _destroyamount (Timeline|DestroyTimeline Stop)
    (:Update
      (Rendering|Material|SetScalarParameterValue (Variables|Default|GetBlocMat) "DestroyAmount" _destroyamount :!class /Script/Engine.MaterialInstanceDynamic))
    (:Finished
      (Actor|DestroyActor))))

(event EventBeginPlay
  (bind _block (Variables|Default|GetBlock))
  (bind _returnvalue (Rendering|Material|CreateDynamicMaterialInstance _block 0 (Rendering|Material|GetMaterial _block 0) "None" :!class /Script/Engine.PrimitiveComponent))
  (Variables|Default|SetBlocMat _returnvalue)
  (Components|Timeline|SetPlayRate (Variables|Default|GetDestroyTimeline) (Variables|Default|GetDestroyRate)))

(fn ConstructionScript)